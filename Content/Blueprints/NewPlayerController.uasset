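; Player controller that lets the player cycle control between three party characters with Q (backward) and E (forward).
; On BeginPlay, after a short delay, it possesses the first character, gives the other two their AI controllers and stores an AI reference on each.
; Each switch copies the new CurrentPossessed index to all characters, hands the previous pawn back to its AI, then calls every character's PersonNPossession handler.
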(event EventBeginPlay
  (bind _character1 (Variables|Default|GetCharacter1))
  (bind _character3 (Variables|Default|GetCharacter3))
  (bind _character2 (Variables|Default|GetCharacter2))
  (Utilities|FlowControl|Delay 0.3)
  (Pawn|Possess (Game|GetPlayerController 0) _character1)
  (Variables|/Game/ThirdPersonBP/Blueprints/ThirdPersonCharacter_1.ThirdPersonCharacter_1_C|SetAI_1 _character1 (Variables|Default|Get1AI))
  (Pawn|Possess (Variables|Default|Get2AI) _character2)
  (Variables|/Game/ThirdPersonBP/Blueprints/ThirdPersonCharacter_2.ThirdPersonCharacter_2_C|SetAI_2 _character2 (Variables|Default|Get2AI))
  (Pawn|Possess (Variables|Default|Get3AI) _character3)
  (Variables|/Game/ThirdPersonBP/Blueprints/ThirdPersonCharacter_3.ThirdPersonCharacter_3_C|SetAI_3 _character3 (Variables|Default|Get3AI))
  (Default|Person3Possession (Variables|Default|GetCharacter3))
  (Default|Person2Possession (Variables|Default|GetCharacter2))
  (Default|Person1Possession (Variables|Default|GetCharacter1)))

(event Input|KeyboardEvents|Q
  (params (Key :type Key%20Structure))
  (:Pressed
    (Variables|Default|SetTemp%20Self%20Ref (Pawn|GetControlledPawn))
    (if (== (Variables|Default|GetCurrentPossessed) 0)
      (bind _output_get (Variables|Default|SetCurrentPossessed 2))
      (Variables|/Game/ThirdPersonBP/Blueprints/ThirdPersonCharacter_1.ThirdPersonCharacter_1_C|SetCurrentPossessed (Variables|Default|GetCharacter1) _output_get)
      (Variables|/Game/ThirdPersonBP/Blueprints/ThirdPersonCharacter_2.ThirdPersonCharacter_2_C|SetCurrentPossessed (Variables|Default|GetCharacter2) _output_get)
      (Variables|/Game/ThirdPersonBP/Blueprints/ThirdPersonCharacter_3.ThirdPersonCharacter_3_C|SetCurrentPossessed (Variables|Default|GetCharacter3) _output_get)
      (Pawn|Possess (Game|GetPlayerController 0) (Variables|Default|GetCharacter3))
      (Pawn|Possess (Variables|/Game/ThirdPersonBP/Blueprints/ThirdPersonCharacter_1.ThirdPersonCharacter_1_C|GetAI_1 (Variables|Default|GetCharacter1)) (Variables|Default|GetTemp%20Self%20Ref))
      (Default|Person3Possession (Variables|Default|GetCharacter3) :!label _label)
      (Default|Person2Possession (Variables|Default|GetCharacter2))
      (Default|Person1Possession (Variables|Default|GetCharacter1))
      (elif (== (Variables|Default|GetCurrentPossessed) 1)
        (bind _output_get_2 (Variables|Default|SetCurrentPossessed 0))
        (Variables|/Game/ThirdPersonBP/Blueprints/ThirdPersonCharacter_1.ThirdPersonCharacter_1_C|SetCurrentPossessed (Variables|Default|GetCharacter1) _output_get_2)
        (Variables|/Game/ThirdPersonBP/Blueprints/ThirdPersonCharacter_2.ThirdPersonCharacter_2_C|SetCurrentPossessed (Variables|Default|GetCharacter2) _output_get_2)
        (Variables|/Game/ThirdPersonBP/Blueprints/ThirdPersonCharacter_3.ThirdPersonCharacter_3_C|SetCurrentPossessed (Variables|Default|GetCharacter3) _output_get_2)
        (Pawn|Possess (Game|GetPlayerController 0) (Variables|Default|GetCharacter1))
        (Pawn|Possess (Variables|/Game/ThirdPersonBP/Blueprints/ThirdPersonCharacter_2.ThirdPersonCharacter_2_C|GetAI_2 (Variables|Default|GetCharacter2)) (Variables|Default|GetTemp%20Self%20Ref))
        (goto _label)
        (elif (== (Variables|Default|GetCurrentPossessed) 2)
          (bind _output_get_3 (Variables|Default|SetCurrentPossessed 1))
          (Variables|/Game/ThirdPersonBP/Blueprints/ThirdPersonCharacter_1.ThirdPersonCharacter_1_C|SetCurrentPossessed (Variables|Default|GetCharacter1) _output_get_3)
          (Variables|/Game/ThirdPersonBP/Blueprints/ThirdPersonCharacter_2.ThirdPersonCharacter_2_C|SetCurrentPossessed (Variables|Default|GetCharacter2) _output_get_3)
          (Variables|/Game/ThirdPersonBP/Blueprints/ThirdPersonCharacter_3.ThirdPersonCharacter_3_C|SetCurrentPossessed (Variables|Default|GetCharacter3) _output_get_3)
          (Pawn|Possess (Game|GetPlayerController 0) (Variables|Default|GetCharacter2))
          (Pawn|Possess (Variables|/Game/ThirdPersonBP/Blueprints/ThirdPersonCharacter_3.ThirdPersonCharacter_3_C|GetAI_3 (Variables|Default|GetCharacter3)) (Variables|Default|GetTemp%20Self%20Ref))
          (goto _label))))))

(event Input|KeyboardEvents|E
  (params (Key :type Key%20Structure))
  (:Pressed
    (Variables|Default|SetTemp%20Self%20Ref (Pawn|GetControlledPawn))
    (if (== (Variables|Default|GetCurrentPossessed) 0)
      (bind _output_get (Variables|Default|SetCurrentPossessed 1))
      (bind _output_get_2 (Variables|/Game/ThirdPersonBP/Blueprints/ThirdPersonCharacter_1.ThirdPersonCharacter_1_C|SetCurrentPossessed (Variables|Default|GetCharacter1) _output_get))
      (bind _output_get_3 (Variables|/Game/ThirdPersonBP/Blueprints/ThirdPersonCharacter_2.ThirdPersonCharacter_2_C|SetCurrentPossessed (Variables|Default|GetCharacter2) _output_get_2))
      (Variables|/Game/ThirdPersonBP/Blueprints/ThirdPersonCharacter_3.ThirdPersonCharacter_3_C|SetCurrentPossessed (Variables|Default|GetCharacter3) _output_get_3)
      (Pawn|Possess (Game|GetPlayerController 0) (Variables|Default|GetCharacter2))
      (Pawn|Possess (Variables|/Game/ThirdPersonBP/Blueprints/ThirdPersonCharacter_1.ThirdPersonCharacter_1_C|GetAI_1 (Variables|Default|GetCharacter1)) (Variables|Default|GetTemp%20Self%20Ref))
      (Default|Person3Possession (Variables|Default|GetCharacter3) :!label _label)
      (Default|Person2Possession (Variables|Default|GetCharacter2))
      (Default|Person1Possession (Variables|Default|GetCharacter1))
      (elif (== (Variables|Default|GetCurrentPossessed) 1)
        (bind _output_get_4 (Variables|Default|SetCurrentPossessed 2))
        (bind _output_get_5 (Variables|/Game/ThirdPersonBP/Blueprints/ThirdPersonCharacter_1.ThirdPersonCharacter_1_C|SetCurrentPossessed (Variables|Default|GetCharacter1) _output_get_4))
        (bind _output_get_6 (Variables|/Game/ThirdPersonBP/Blueprints/ThirdPersonCharacter_2.ThirdPersonCharacter_2_C|SetCurrentPossessed (Variables|Default|GetCharacter2) _output_get_5))
        (Variables|/Game/ThirdPersonBP/Blueprints/ThirdPersonCharacter_3.ThirdPersonCharacter_3_C|SetCurrentPossessed (Variables|Default|GetCharacter3) _output_get_6)
        (Pawn|Possess (Game|GetPlayerController 0) (Variables|Default|GetCharacter3))
        (Pawn|Possess (Variables|/Game/ThirdPersonBP/Blueprints/ThirdPersonCharacter_2.ThirdPersonCharacter_2_C|GetAI_2 (Variables|Default|GetCharacter2)) (Variables|Default|GetTemp%20Self%20Ref))
        (goto _label)
        (elif (== (Variables|Default|GetCurrentPossessed) 2)
          (bind _output_get_7 (Variables|Default|SetCurrentPossessed 0))
          (bind _output_get_8 (Variables|/Game/ThirdPersonBP/Blueprints/ThirdPersonCharacter_1.ThirdPersonCharacter_1_C|SetCurrentPossessed (Variables|Default|GetCharacter1) _output_get_7))
          (bind _output_get_9 (Variables|/Game/ThirdPersonBP/Blueprints/ThirdPersonCharacter_2.ThirdPersonCharacter_2_C|SetCurrentPossessed (Variables|Default|GetCharacter2) _output_get_8))
          (Variables|/Game/ThirdPersonBP/Blueprints/ThirdPersonCharacter_3.ThirdPersonCharacter_3_C|SetCurrentPossessed (Variables|Default|GetCharacter3) _output_get_9)
          (Pawn|Possess (Game|GetPlayerController 0) (Variables|Default|GetCharacter1))
          (Pawn|Possess (Variables|/Game/ThirdPersonBP/Blueprints/ThirdPersonCharacter_3.ThirdPersonCharacter_3_C|GetAI_3 (Variables|Default|GetCharacter3)) (Variables|Default|GetTemp%20Self%20Ref))
          (goto _label))))))

(fn ConstructionScript)